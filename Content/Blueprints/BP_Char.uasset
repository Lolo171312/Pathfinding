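; BP_Char is a player Blueprint that views the game through a camera placed in the level, with a visible mouse cursor.
; On BeginPlay it finds a CameraActor, sets it as player 0's view target and shows the cursor.
; A disconnected chain that would possess the actor and add the IMC_inputs Enhanced Input mapping context never runs.
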(event `self.ReceiveBeginPlay`
  (bind _returnvalue (`GameplayStatics.GetPlayerController` 0))
  (bind _returnvalue_2 (`GameplayStatics.GetActorOfClass` "/Script/Engine.CameraActor"))
  (`PlayerController.SetViewTargetWithBlend` _returnvalue _returnvalue_2 0.0 "VTBlend_Linear" 0.0 false)
  (set `PlayerController.bShowMouseCursor` true _returnvalue))

(fn `UserConstructionScript`)